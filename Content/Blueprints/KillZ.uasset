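; KillZ is a placeable kill plane that kills any ThirdPersonCharacter at or below its own height.
; Each Tick it gathers every ThirdPersonCharacter with GetAllActorsOfClass and compares their Z location to the actor's, with no overlap volume involved.
; Characters at or below that height that are not already in the "die" state are switched to it through SwitchState.
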(event EventBeginPlay)

(event Collision|EventActorBeginOverlap
  (params (OtherActor :type Actor%20Object%20Reference)))

(event EventTick
  (params (DeltaSeconds :type Float%20%28single-precision%29))
  (bind _outactors (Actor|GetAllActorsOfClass "/Game/Blueprints/Character/ThirdPersonCharacter.ThirdPersonCharacter_C"))
  (for _array_element _outactors
    (if (and (<= (.Z (Math|Vector|BreakVector (Transformation|GetActorLocation _array_element))) (.Z (Math|Vector|BreakVector (Transformation|GetActorLocation)))) (Utilities|Enum|NotEqual(Enum) (Variables|/Game/Blueprints/Character/ThirdPersonCharacter.ThirdPersonCharacter_C|GetCurrentState _array_element) "die"))
      (Default|SwitchState _array_element "die"))))

(fn ConstructionScript)