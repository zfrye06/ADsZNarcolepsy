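; PA speaker actor that periodically launches SocialInteraction actors from its LaunchPos point.
; A Tick-driven timer spawns each one once the launch delay passes, plays a radio "wah" sound and triggers a jiggle.
; The jiggle resets a second timer, which drives an elastic ease-out uniform scale on the Speaker component every frame for a bouncy pulse.
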(event Custom|Jiggle
  (Variables|Default|SetJiggleTimer 0.0))

(event EventTick
  (params (DeltaSeconds :type Float%20%28single-precision%29))
  (Utilities|JiggleLogic DeltaSeconds)
  (if (<= (Variables|Default|GetLaunchTimer) (Variables|Default|GetLaunchDelay))
    (Variables|Default|SetLaunchTimer (+ (Variables|Default|GetLaunchTimer) DeltaSeconds))
    (else
      (Variables|Default|SetLaunchTimer 0.0)
      (Game|SpawnActorfromClass "/Game/Blueprints/SocialInteraction.SocialInteraction_C" (Transformation|GetWorldTransform (Variables|Default|GetLaunchPos)) "Undefined" 0 0)
      (Audio|PlaySoundatLocation "/Game/Sounds/radio_wah.radio_wah" (Transformation|GetActorLocation))
      (CallFunction|Jiggle))))

(fn ConstructionScript)