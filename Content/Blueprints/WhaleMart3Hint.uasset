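; WhaleMart3Hint is a proximity trigger that shows an on-screen hint while the third-person character is inside its sphere.
; On overlap begin, it lazily creates the HintWB widget for player 0, caches it, and adds it to the viewport.
; On overlap end, it removes the cached widget from the screen and keeps the reference for reuse on later entries.
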(event OnComponentBeginOverlap(Sphere)
  (params (OverlappedComponent :type Primitive%20Component%20Object%20Reference) (OtherActor :type Actor%20Object%20Reference) (OtherComp :type Primitive%20Component%20Object%20Reference) (OtherBodyIndex :type Integer) (bFromSweep :type Boolean) (SweepResult :type Hit%20Result%20Structure%20%28by%20ref%29))
  (Utilities|Casting|CastToThirdPersonCharacter OtherActor)
  (Utilities|IsValid (Variables|Default|GetHintWB)
    (:Is%20Valid
      _)
    (:Is%20Not%20Valid
      (bind _returnvalue (UserInterface|CreateWidget "/Game/Blueprints/UI/HintWB.HintWB_C" (Game|GetPlayerController 0)))
      (Variables|Default|SetHintWB _returnvalue)))
  (UserInterface|Viewport|AddtoViewport (Variables|Default|GetHintWB) 0))

(event OnComponentEndOverlap(Sphere)
  (params (OverlappedComponent :type Primitive%20Component%20Object%20Reference) (OtherActor :type Actor%20Object%20Reference) (OtherComp :type Primitive%20Component%20Object%20Reference) (OtherBodyIndex :type Integer))
  (Utilities|Casting|CastToThirdPersonCharacter OtherActor)
  (Utilities|IsValid (Variables|Default|GetHintWB)
    (:Is%20Valid
      (Widget|RemovefromParent (Variables|Default|GetHintWB)))))

(event EventBeginPlay)

(event Collision|EventActorBeginOverlap
  (params (OtherActor :type Actor%20Object%20Reference)))

(event EventTick
  (params (DeltaSeconds :type Float%20%28single-precision%29)))

(fn ConstructionScript)