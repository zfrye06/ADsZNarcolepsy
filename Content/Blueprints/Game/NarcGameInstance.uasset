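; Game instance that manages the NarcSaveGame slot and player respawning.
; On Init it loads an existing save, or otherwise calls CreateSaveGame (an empty stub here), runs a hardware benchmark and writes the slot.
; SaveSaveGame writes the held save object back to that slot.
; RespawnPlayer destroys the controlled pawn, spawns and possesses a new ThirdPersonCharacter at the first PlayerStart found, and restores game-only input.
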(event Custom|RespawnPlayer
  (bind _returnvalue (Game|GetPlayerController 0))
  (Actor|DestroyActor (Pawn|GetControlledPawn (Game|GetPlayerController 0)))
  (bind _outactors (Actor|GetAllActorsOfClass "/Script/Engine.PlayerStart"))
  (bind _returnvalue_2 (Game|SpawnActorfromClass "/Game/Blueprints/Character/ThirdPersonCharacter.ThirdPersonCharacter_C" (Transformation|GetActorTransform (Utilities|Array|Get(acopy) _outactors)) "Undefined" 0 0))
  (Pawn|Possess _returnvalue _returnvalue_2)
  (Input|SetInputModeGameOnly _returnvalue)
  (Variables|/Script/Engine.PlayerController|SetbShowMouseCursor _returnvalue false))

(event EventInit
  ;[1 0.1817 0] Game Instance Game Startup. Creates save game or loads it
  (bind _returnvalue (SaveGame|DoesSaveGameExist (Variables|Default|GetSaveSlot)))
  (if _returnvalue
    (CallFunction|LoadSaveGame)
    (else
      ;;[0.1354 1 0] Runs a hardware benchmark if user is starting the game for the first time
      (CallFunction|CreateSaveGame)
      (bind _returnvalue_2 (Settings|GetGameUserSettings))
      (Class|GameUserSettings|RunHardwareBenchmark _returnvalue_2 10 1.0 1.0)
      (SaveGame|SaveGametoSlot (Variables|Default|GetSaveGame) (Variables|Default|GetSaveSlot)))))

(fn CreateSaveGame)

(fn LoadSaveGame
  (bind _returnvalue (SaveGame|LoadGamefromSlot (Variables|Default|GetSaveSlot)))
  (bind _asnarc_save_game (Utilities|Casting|CastToNarcSaveGame _returnvalue))
  (Variables|Default|SetSaveGame _asnarc_save_game))

(fn SaveSaveGame
  (SaveGame|SaveGametoSlot (Variables|Default|GetSaveGame) (Variables|Default|GetSaveSlot)))