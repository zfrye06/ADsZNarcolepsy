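; IceCream is a level-goal pickup that bobs and spins until a living ThirdPersonCharacter overlaps its sphere.
; The overlap shows a PickUp widget and starts a timed, elastic-eased scale animation.
; When the timer ends, it plays a sound, hides the mesh and waits briefly.
; It then opens the game instance's NextLevel, or shows the WinScreen with a mouse cursor if that level is MainMenu.
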(event OnComponentBeginOverlap(Sphere)
  (params (OverlappedComponent :type Primitive%20Component%20Object%20Reference) (OtherActor :type Actor%20Object%20Reference) (OtherComp :type Primitive%20Component%20Object%20Reference) (OtherBodyIndex :type Integer) (bFromSweep :type Boolean) (SweepResult :type Hit%20Result%20Structure%20%28by%20ref%29))
  (bind _asthird_person_character (Utilities|Casting|CastToThirdPersonCharacter OtherActor))
  (if (not (Variables|/Game/Blueprints/Character/ThirdPersonCharacter.ThirdPersonCharacter_C|GetIsDead _asthird_person_character))
    (Variables|Default|SetGrabbed true)
    (bind _returnvalue (UserInterface|CreateWidget "/Game/Blueprints/UI/PickUp.PickUp_C" (Game|GetPlayerController 0)))
    (bind _output_get (Variables|Default|SetPickUpWB _returnvalue))
    (UserInterface|Viewport|AddtoViewport _returnvalue 0)))

(event EventBeginPlay
  (Variables|Default|SetCurrentPos (Transformation|GetActorLocation)))

(event EventTick
  (params (DeltaSeconds :type Float%20%28single-precision%29))
  (bind _returnvalue (Transformation|GetActorRotation))
  (bind _currentpos (Variables|Default|GetCurrentPos))
  (bind (_roll _pitch _yaw) (Math|Rotator|BreakRotator _returnvalue))
  (bind (_x _y _z) (Math|Vector|BreakVector _currentpos))
  (if (Variables|Default|GetGrabbed)
    (bind (_progress _done) (CallFunction|TimerIncrement (Variables|Default|GetDelayGrabTimer) (Variables|Default|GetDelayGrabLength) DeltaSeconds))
    (bind _returnvalue_2 (CallFunction|EaseElasticin _progress 1.0))
    (Transformation|SetActorScale3D (Math|Vector|MakeVector (+ _returnvalue_2 1.0) (+ _returnvalue_2 1.0) (+ _returnvalue_2 1.0)))
    (if _done
      (if (Variables|Default|GetPlayedSound)
        _
        (else
          (Audio|PlaySoundatLocation "/Game/Sounds/scarf.scarf" (Transformation|GetActorLocation))
          (Variables|Default|SetPlayedSound true)))
      (Rendering|SetVisibility (Variables|Default|GetStaticMesh) false false)
      (Utilities|FlowControl|Delay 1.0)
      (bind _asnarc_game_instance (Utilities|Casting|CastToNarcGameInstance (Game|GetGameInstance)))
      (if (Utilities|Name|Equal(Name) (Variables|/Game/Blueprints/Game/NarcGameInstance.NarcGameInstance_C|GetNextLevel _asnarc_game_instance) (Utilities|Name|MakeLiteralName "MainMenu"))
        (Widget|RemovefromParent (Variables|Default|GetPickUpWB))
        (bind _returnvalue_3 (UserInterface|CreateWidget "/Game/Blueprints/UI/WinScreen.WinScreen_C" (Game|GetPlayerController 0)))
        (UserInterface|Viewport|AddtoViewport _returnvalue_3 0)
        (Variables|/Script/Engine.PlayerController|SetbShowMouseCursor (Game|GetPlayerController 0) true)
        (else
          (Widget|RemovefromParent (Variables|Default|GetPickUpWB))
          (Game|OpenLevel(byName) (Variables|/Game/Blueprints/Game/NarcGameInstance.NarcGameInstance_C|GetNextLevel _asnarc_game_instance)))))
    (else
      ;[1 1 1] Float and rotate
      (bind _output_get (Variables|Default|SetTimer (+ (Variables|Default|GetTimer) DeltaSeconds)))
      (Transformation|SetActorLocation (Math|Vector|MakeVector _x _y (+ _z (* (Math|Trig|Sin(Radians) _output_get) (Variables|Default|GetFloatVariance)))) false true)
      (Transformation|SetActorRotation (Math|Rotator|MakeRotator _roll _pitch (+ _yaw (* DeltaSeconds 1e+02)))))))

(fn ConstructionScript)