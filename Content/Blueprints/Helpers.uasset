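; Helper functions for advancing timers and for scaling scene components around their actor's origin.
; TimerIncrement adds delta time to a by-ref timer, returning progress and flagging done on a call that finds it at or past its length, where it clamps.
; ScaleAroundActorOrigin sets relative scale, then multiplies the saved relative location by new over current scale, read after the change.
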(fn TimerIncrement
  (params (Timer :type Float%20%28single-precision%29%20%28by%20ref%29) (Length :type Float%20%28single-precision%29) (DT :type Float%20%28single-precision%29))
  (if (< Timer Length)
    (|SetBy-RefVar Timer (+ Timer DT))
    (else
      (|SetBy-RefVar Timer Length)
      (LocalVariables|SetDoneSet true)))
  (return (/ Timer Length) (LocalVariables|GetDoneSet)))

(fn ScaleAroundActorOrigin
  (params (Target :type Scene%20Component%20Object%20Reference) (Scale :type Vector) (bTeleport :type Boolean))
  (LocalVariables|SetSaveTransform (Variables|/Script/Engine.SceneComponent|GetRelativeLocation Target))
  (Transformation|SetRelativeScale3D Target Scale)
  (Transformation|SetRelativeLocation Target (* (LocalVariables|GetSaveTransform) (/ Scale (Variables|/Script/Engine.SceneComponent|GetRelativeScale3D Target))) false bTeleport))