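; Granny enemy that turns toward the player, fires SocialInteraction actors, and smashes the player away on overlap or hit.
; A Tick-driven state machine (Idle, Lookat, Pause, Smash) uses SwitchState for entry effects and TargetInRange to choose transitions.
; Lookat turns yaw with cubic ease-in, then Pause spawns the actor from the player-aimed FireLocation and waits.
; Smash plays a sound and keeps facing the player until its lag timer ends.
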(event EventBeginPlay
  (Variables|Default|SetTarget (Game|Player|GetPlayerPawn 0))
  (Variables|Default|SetOriginalRotation (Transformation|GetActorRotation)))

(event Collision|EventActorBeginOverlap
  (params (OtherActor :type Actor%20Object%20Reference))
  (bind _asthird_person_character (Utilities|Casting|CastToThirdPersonCharacter OtherActor))
  (Default|Smash _asthird_person_character (* (- (Transformation|GetActorLocation) (Transformation|GetActorLocation _asthird_person_character)) (Variables|Default|GetSmashImpulseMultiplier)))
  (CallFunction|SwitchState "smash"))

(event Collision|EventHit
  (params (MyComp :type Primitive%20Component%20Object%20Reference) (Other :type Actor%20Object%20Reference) (OtherComp :type Primitive%20Component%20Object%20Reference) (bSelfMoved :type Boolean) (HitLocation :type Vector :default "0, 0, 0") (HitNormal :type Vector) (NormalImpulse :type Vector :default "0, 0, 0") (Hit :type Hit%20Result%20Structure%20%28by%20ref%29))
  (bind _asthird_person_character (Utilities|Casting|CastToThirdPersonCharacter Other))
  (Default|Smash _asthird_person_character (* (Math|Vector|NegateVector HitNormal) (Variables|Default|GetSmashImpulseMultiplier)))
  (CallFunction|SwitchState "smash"))

(event EventTick
  (params (DeltaSeconds :type Float%20%28single-precision%29))
  (Variables|Default|SetDT DeltaSeconds)
  (Transformation|SetWorldRotation (Variables|Default|GetFireLocation) (Math|Rotator|FindLookatRotation (Transformation|GetWorldLocation (Variables|Default|GetFireLocation)) (Transformation|GetActorLocation (Variables|Default|GetTarget))) false false)
  (switch string (Variables|Default|GetCurrentState)
    (:Default
      (if (Utilities|TargetinRange) :!label _label
        (CallFunction|SwitchState "lookat")))
    (:idle
      (goto _label))
    (:lookat
      (bind _finished (CallFunction|EaseRotateTowards (Math|Rotator|MakeRotator 0.0 0.0 (.Yaw (Math|Rotator|BreakRotator (Math|Rotator|FindLookatRotation (Transformation|GetActorLocation) (Transformation|GetActorLocation (Variables|Default|GetTarget)))))) (Variables|Default|GetOriginalRotation) (Variables|Default|GetDT)))
      (if _finished
        (CallFunction|SwitchState "pause")))
    (:pause
      (bind _done (CallFunction|TimerIncrement (Variables|Default|GetDelayTimer) (Variables|Default|GetDelayAfterFiring) (Variables|Default|GetDT)))
      (if _done
        (if (Utilities|TargetinRange)
          (CallFunction|SwitchState "lookat")
          (else
            (CallFunction|SwitchState "idle")))))
    (:smash
      (bind _done_2 (CallFunction|TimerIncrement (Variables|Default|GetSmashTimer) (Variables|Default|GetSmashLagLength) (Variables|Default|GetDT)))
      (if _done_2
        (if (Utilities|TargetinRange)
          (CallFunction|SwitchState "lookat")
          (else
            (CallFunction|SwitchState "idle")))
        (else
          (Transformation|SetActorRotation (Math|Rotator|MakeRotator 0.0 0.0 (.Yaw (Math|Rotator|BreakRotator (Math|Rotator|FindLookatRotation (Transformation|GetActorLocation) (Transformation|GetActorLocation (Variables|Default|GetTarget))))))))))))

(fn ConstructionScript)

(fn SwitchState
  (params (NewState :type String))
  (switch string (Variables|Default|GetCurrentState) ; deinit
    (:Default
      _)
    (:lookat
      _))
  (bind _output_get (Variables|Default|SetCurrentState NewState))
  (switch string _output_get ; init
    (:lookat
      (Variables|Default|SetLookAtTimer 0.0)
      (Variables|Default|SetOriginalRotation (Transformation|GetActorRotation)))
    (:pause
      (Game|SpawnActorfromClass "/Game/Blueprints/SocialInteraction.SocialInteraction_C" (Transformation|GetWorldTransform (Variables|Default|GetFireLocation)) "Undefined" 0 self)
      (Audio|PlaySoundatLocation "/Game/Sounds/wah.wah" (Transformation|GetActorLocation))
      (Variables|Default|SetDelayTimer 0.0))
    (:smash
      (Variables|Default|SetSmashTimer 0.0)
      (Audio|PlaySoundatLocation "/Game/Sounds/smack.smack" (Transformation|GetActorLocation)))))

(fn EaseRotateTowards
  (params (Target :type Rotator) (Original :type Rotator) (dt :type Float%20%28single-precision%29))
  (if (<= (Variables|Default|GetLookAtTimer) (Variables|Default|GetLookAtLength))
    (bind _output_get (Variables|Default|SetLookAtTimer (+ (Variables|Default|GetLookAtTimer) dt)))
    (else
      (Variables|Default|SetLookAtTimer (Variables|Default|GetLookAtLength))
      (LocalVariables|SetDone true)))
  (bind _returnvalue (CallFunction|EaseCubicin (/ _output_get (Variables|Default|GetLookAtLength))))
  (Transformation|SetActorRotation (Math|Rotator|CombineRotators (* Original (- 1.0 _returnvalue)) (* Target _returnvalue)))
  (return (LocalVariables|GetDone)))