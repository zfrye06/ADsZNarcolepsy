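; Enemy cart hazard that rolls along a looping spline and smashes the third-person character on contact.
; Tick advances distance along CartPath from a random start, placing the mesh with a rotation offset plus slight random jitter for rattle.
; Overlap and hit events call the character's Smash with a scaled impulse from relative position or hit normal.
; A rolling sound follows the mesh, and a smack sound plays on contact.
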(event EventBeginPlay
  (Audio|SpawnSoundAttached "/Game/Sounds/rolling_cart_cue.rolling_cart_cue" (Variables|Default|GetStaticMesh) "None" "0, 0, 0" "0, 0, 0" "KeepRelativeOffset" true)
  (Variables|Default|SetCartPosition (Math|Random|RandomFloatinRange 0.0 (Spline|GetSplineLength (Variables|Default|GetCartPath)))))

(event Collision|EventActorBeginOverlap
  (params (OtherActor :type Actor%20Object%20Reference))
  (bind _asthird_person_character (Utilities|Casting|CastToThirdPersonCharacter OtherActor))
  (Default|Smash _asthird_person_character (* (- (Transformation|GetActorLocation) (Transformation|GetActorLocation _asthird_person_character)) (Variables|Default|GetSmashImpulseMultiplier)))
  (Audio|SpawnSoundatLocation "/Game/Sounds/cart_smack.cart_smack" (Transformation|GetActorLocation)))

(event Collision|EventHit
  (params (MyComp :type Primitive%20Component%20Object%20Reference) (Other :type Actor%20Object%20Reference) (OtherComp :type Primitive%20Component%20Object%20Reference) (bSelfMoved :type Boolean) (HitLocation :type Vector) (HitNormal :type Vector) (NormalImpulse :type Vector :default "0, 0, 0") (Hit :type Hit%20Result%20Structure%20%28by%20ref%29))
  (bind _asthird_person_character (Utilities|Casting|CastToThirdPersonCharacter Other))
  (Default|Smash _asthird_person_character (* (Math|Vector|NegateVector HitNormal) (Variables|Default|GetSmashImpulseMultiplier)))
  (Audio|SpawnSoundatLocation "/Game/Sounds/cart_smack.cart_smack" HitLocation))

(event EventTick
  (params (DeltaSeconds :type Float%20%28single-precision%29))
  (bind _cartpath (Variables|Default|GetCartPath))
  (bind _staticmesh (Variables|Default|GetStaticMesh))
  ;[1 1 1] Cart Follows Along Spline
  (Variables|Default|SetCartPosition (+ (* DeltaSeconds (Variables|Default|GetMovementSpeed)) (Variables|Default|GetCartPosition)))
  (Transformation|SetWorldLocation _staticmesh (Spline|GetLocationatDistanceAlongSpline _cartpath (Variables|Default|GetCartPosition) "World") false false)
  (Transformation|SetWorldRotation _staticmesh (Math|Rotator|CombineRotators (Math|Rotator|CombineRotators (Spline|GetRotationatDistanceAlongSpline _cartpath (Variables|Default|GetCartPosition) "World") "0,159.000000, 0") (* (Math|Random|RandomRotator true) 0.005)) false false)
  (if (> (Variables|Default|GetCartPosition) (Spline|GetSplineLength (Variables|Default|GetCartPath))) ; Restart back at the beginning of the spline if we've run out of spline
    (Variables|Default|SetCartPosition 0.0)))

(fn ConstructionScript)