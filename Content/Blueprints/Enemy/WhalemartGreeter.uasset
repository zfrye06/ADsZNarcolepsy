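; Whalemart greeter enemy that turns toward the player and fires a single SocialInteraction actor, gated by a TargetInRange check.
; A Tick-driven state machine runs Idle, Lookat, Pause and Finish, turning back to its starting rotation after a delay.
; SwitchState handles exit and entry logic, spawning the shot at FireLocation on leaving Lookat and setting Fired to prevent repeats.
; EaseRotateTowards blends rotations with a timed cubic ease-in.
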(event EventBeginPlay
  (Variables|Default|SetTarget (Game|Player|GetPlayerPawn 0))
  (Variables|Default|SetOriginalRotation (Transformation|GetActorRotation)))

(event Collision|EventActorBeginOverlap
  (params (OtherActor :type Actor%20Object%20Reference)))

(event EventTick
  (params (DeltaSeconds :type Float%20%28single-precision%29))
  (switch string (Variables|Default|GetCurrentState)
    (:idle
      (if (and (Utilities|TargetinRange) (not (Variables|Default|GetFired)))
        (CallFunction|SwitchState "lookat")))
    (:lookat
      (bind _finished (CallFunction|EaseRotateTowards (Math|Rotator|MakeRotator 0.0 0.0 (.Yaw (Math|Rotator|BreakRotator (Math|Rotator|FindLookatRotation (Transformation|GetActorLocation) (Transformation|GetActorLocation (Variables|Default|GetTarget)))))) (Variables|Default|GetOriginalRotation) DeltaSeconds))
      (if _finished
        (CallFunction|SwitchState "pause")))
    (:finish
      (bind _finished_2 (CallFunction|EaseRotateTowards (Variables|Default|GetOriginalRotation) (Variables|Default|GetRotationSave) DeltaSeconds))
      (if _finished_2
        (CallFunction|SwitchState "idle")))
    (:pause
      (if (<= (Variables|Default|GetDelayTimer) (Variables|Default|GetDelayAfterFiring))
        (Variables|Default|SetDelayTimer (+ (Variables|Default|GetDelayTimer) DeltaSeconds))
        (else
          (CallFunction|SwitchState "finish"))))))

(fn ConstructionScript)

(fn SwitchState
  (params (NewState :type String))
  (switch string (Variables|Default|GetCurrentState) ; deinit
    (:Default
      _)
    (:lookat
      (Game|SpawnActorfromClass "/Game/Blueprints/SocialInteraction.SocialInteraction_C" (Transformation|GetWorldTransform (Variables|Default|GetFireLocation)) "Undefined" 0 self)
      (Variables|Default|SetFired true)))
  (bind _output_get (Variables|Default|SetCurrentState NewState))
  (switch string _output_get ; init
    (:finish
      (Variables|Default|SetRotationSave (Transformation|GetActorRotation))
      (Variables|Default|SetLookAtTimer 0.0))
    (:lookat
      (Variables|Default|SetLookAtTimer 0.0))
    (:pause
      (Variables|Default|SetDelayTimer 0.0))))

(fn EaseRotateTowards
  (params (Target :type Rotator) (Original :type Rotator) (dt :type Float%20%28single-precision%29))
  (if (<= (Variables|Default|GetLookAtTimer) (Variables|Default|GetLookAtLength))
    (bind _output_get (Variables|Default|SetLookAtTimer (+ (Variables|Default|GetLookAtTimer) dt)))
    (else
      (Variables|Default|SetLookAtTimer (Variables|Default|GetLookAtLength))
      (LocalVariables|SetDone true)))
  (bind _returnvalue (CallFunction|EaseCubicin (/ _output_get (Variables|Default|GetLookAtLength))))
  (Transformation|SetActorRotation (Math|Rotator|CombineRotators (* Original (- 1.0 _returnvalue)) (* Target _returnvalue)))
  (return (LocalVariables|GetDone)))